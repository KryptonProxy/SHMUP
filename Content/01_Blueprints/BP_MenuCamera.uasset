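; BP_MenuCamera is an actor Blueprint that brings up the main menu when play begins.
; On BeginPlay, if its Menu reference is not valid, it removes all widgets and creates a BPW_MainMenu.
; It then gives the PlayButton keyboard focus, switches the player controller to UI-only input, adds the menu to the viewport and shows the mouse cursor.
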(event `self.ReceiveBeginPlay`
  (bind _returnvalue (`GameplayStatics.GetPlayerController` 0))
  (bind _playbutton (`/Game/07_UI/BPW_MainMenu.PlayButton` (`self.Menu`)))
  (`self.Menu`
    (:`then`
      _)
    (:`else`
      (`WidgetLayoutLibrary.RemoveAllWidgets`)
      (bind _returnvalue_2 (`|CreateWidget` "/Game/07_UI/BPW_MainMenu.BPW_MainMenu_C"))
      (set `self.Menu` _returnvalue_2)))
  (`Widget.SetKeyboardFocus` _playbutton)
  (`WidgetBlueprintLibrary.SetInputMode_UIOnlyEx` _returnvalue _playbutton)
  (`UserWidget.AddToViewport` (`self.Menu`) 1)
  (set `PlayerController.bShowMouseCursor` true _returnvalue))

(fn `UserConstructionScript`)