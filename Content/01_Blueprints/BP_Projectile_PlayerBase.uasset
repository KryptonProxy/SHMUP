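; BP_Projectile_PlayerBase is, by its name, the base player projectile, with configurable color, scale and initial speed.
; The construction script creates a dynamic glow material instance on the Projectile component, scales that component and passes the speed to ProjectileMovement.
; BeginPlay then applies the color to the material's Color parameter.
; The node that would match MaxSpeed to InitialSpeed is disconnected, and no overlap or damage logic exists here.
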(event `self.ReceiveBeginPlay`
  (`MaterialInstanceDynamic.SetVectorParameterValue` (`self.ProjectileMaterial`) "Color" (`self.ProjectileColor`)))

(fn `UserConstructionScript`
  (bind _returnvalue (`PrimitiveComponent.CreateDynamicMaterialInstance` (`self.Projectile`) 0 "/Game/03_Materials/Glow/M_Glow_Projectile.M_Glow_Projectile" "None"))
  (set `self.ProjectileMaterial` _returnvalue)
  (`SceneComponent.SetWorldScale3D` (`self.Projectile`) (`self.Scale`))
  (bind _output_get (set `ProjectileMovementComponent.InitialSpeed` (`self.Initial Speed`) (`self.ProjectileMovement`))))