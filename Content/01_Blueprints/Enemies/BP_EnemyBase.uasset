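; Base enemy Blueprint for a shoot 'em up, providing spawn entry and horizontal movement.
; On BeginPlay it increments the enemy count in BP_SHMUP, picks a random direction and speed, and caches its spawn location.
; A timeline lowers it along Z from that location, then enables movement when finished.
; Tick then moves it along X without sweeping, with no bounds check or direction change.
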(event `self.ReceiveBeginPlay`
  (bind _spawnlocation (`self.SpawnLocation`))
  ;[1 1 1] Setup Refs & Var
  (bind _asbp_shmup (cast `/Game/01_Blueprints/BP_SHMUP` (`GameplayStatics.GetGameMode`)))
  (bind _output_get (set `self.BP_GameMode` _asbp_shmup))
  (`/Game/01_Blueprints/BP_SHMUP.UpdateEnemyCount` _output_get 1)
  (set `self.MoveDirection` (`KismetMathLibrary.RandomBool`))
  (set `self.MoveSpeed` (`KismetMathLibrary.RandomFloatInRange` (`self.MinSpeed`) (`self.MaxSpeed`)))
  (set `self.SpawnLocation` (`self.K2_GetActorLocation`))
  ;[1 1 1] Spawn Anim
  (bind (_direction _entryspeed) (`Timeline|SpawnAnimation`)
    (:`Update`
      (`self.K2_SetActorLocation` (`KismetMathLibrary.VLerp` _spawnlocation (- _spawnlocation (0.0 0.0 120.0)) _entryspeed)))
    (:`Finished`
      (set `self.MoveEnabled` true))))

(event `self.ReceiveTick`
  (params (DeltaSeconds :type "Float (single-precision)"))
  (if (`self.MoveEnabled`)
    (`self.K2_SetActorLocation` (+ (`self.K2_GetActorLocation`) (* (`KismetMathLibrary.MakeVector` (* (`self.MoveSpeed`) (`KismetMathLibrary.SelectFloat` 1.0 -1.0 (`self.MoveDirection`)))) DeltaSeconds)))))

(fn `UserConstructionScript`)